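; Table tennis ball that launches itself toward a fixed target point when a racket hits it.
; BeginPlay caches the location of a referenced actor as the target.
; On a mesh hit from BP_Racket, it solves a custom-arc projectile velocity to that point and, on success, replaces the ball's physics linear velocity.
; Each racket hit also draws a debug line from the ball to the raw impact normal value.
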(event `self.ReceiveBeginPlay`
  (set `self.TargetPosition` (`self.K2_GetActorLocation` (`self.NewVar`))))

(event `self.BallMesh.OnComponentHit`
  (params (HitComponent :type "PrimitiveComponent Object Reference") (OtherActor :type "Actor Object Reference") (OtherComp :type "PrimitiveComponent Object Reference") (NormalImpulse :type "Vector Structure") (Hit :type "HitResult Structure (by ref)"))
  (bind _returnvalue (`self.K2_GetActorLocation`))
  (cast `/Game/TableTennis/BP_Racket` OtherActor)
  (`KismetSystemLibrary.DrawDebugLine` _returnvalue Hit_ImpactNormal (struct :`R` 0.220737 :`B` 1.0 :`A` 1.0) 10.0 5.0)
  (bind (_outlaunchvelocity _returnvalue_2) (`GameplayStatics.SuggestProjectileVelocity_CustomArc` _returnvalue (`self.TargetPosition`)))
  (if _returnvalue_2
    (`PrimitiveComponent.SetPhysicsLinearVelocity` (`self.BallMesh`) _outlaunchvelocity false "None")))

(fn `UserConstructionScript`)