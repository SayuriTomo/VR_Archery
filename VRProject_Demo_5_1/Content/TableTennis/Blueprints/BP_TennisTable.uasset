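; BP_TennisTable is the table tennis table actor, which manages the game's start menu.
; On BeginPlay it binds to PlayerRacket's open and close start-widget dispatchers, spawning a Menu actor if none exists or closing the current one.
; StartGame closes a valid menu and plays a 2D sound, with no further game logic here.
; Unconnected VRPawn menu-toggle nodes remain in the graph and never run.
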(event `self.ReceiveBeginPlay`
  (bind _player_racket (`self.Player_Racket`))
  (add `/Game/TableTennis/Blueprints/BP_Racket.OnOpenStartWidgetEventDispatcher` _player_racket (delegate `OpenStartWidget`))
  (add `/Game/TableTennis/Blueprints/BP_Racket.OnCloseStartWidgetEventDispatcher` _player_racket (delegate `CloseStartWidget`)))

(event `OpenStartWidget`
  (`self.ToggleMenu`))

(event `CloseStartWidget`
  (bind _menureference (`self.MenuReference`)
    (:`then`
      (`/Game/TableTennis/Widget/Menu.CloseMenu` _menureference))
    (:`else`)))

(fn `Start Game`
  (bind _menureference (`self.MenuReference`)
    (:`then`
      (`/Game/TableTennis/Widget/Menu.CloseMenu` _menureference)
      (`GameplayStatics.PlaySound2D` "/Game/StarterContent/Audio/Collapse01.Collapse01" 1.0 1.0 0.0 null null))
    (:`else`)))

(fn `ToggleMenu`
  (`self.MenuReference`
    (:`then`)
    (:`else`
      (bind _returnvalue (`|SpawnActorFromClass` "/Game/TableTennis/Widget/Menu.Menu_C" (`KismetMathLibrary.MakeTransform` (0.0 0.0 0.0)) "Undefined" "OverrideRootScale" null false self))
      (set `self.MenuReference` _returnvalue))))

(fn `UserConstructionScript`)