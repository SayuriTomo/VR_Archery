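; BP_Racket is a grabbable table tennis racket that opens a start widget when grabbed, and closes it and returns to its spawn transform when dropped.
; Tick derives swing velocity and speed from frame-to-frame movement.
; When its box hits a BP_TennisBall, scaled swing speed feeds a high-arc projectile velocity solve toward a target actor, overriding the ball's physics velocity if a solution exists.
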(event `self.ReceiveBeginPlay`
  (set `self.StartPosition` (`self.GetTransform`)))

(event `self.GrabComponent.OnDropped`
  (`SceneComponent.K2_SetWorldTransform` (`self.RacketMesh`) (`self.StartPosition`) false false)
  (`self.OnCloseStartWidgetEventDispatcher`))

(event `self.GrabComponent.OnGrabbed`
  (`self.OnOpenStartWidgetEventDispatcher`))

(event `self.ReceiveTick`
  (params (DeltaSeconds :type "Float (single-precision)"))
  (bind _returnvalue (`self.K2_GetActorLocation`))
  (bind _output_get (set `self.SwingVelocity` (/ (- _returnvalue (`self.PreviousLocation`)) DeltaSeconds)))
  (set `self.SwingSpeed` (`KismetMathLibrary.VSize` _output_get))
  (set `self.PreviousLocation` _returnvalue))

(event `self.Box.OnComponentHit`
  (params (HitComponent :type "PrimitiveComponent Object Reference") (OtherActor :type "Actor Object Reference") (OtherComp :type "PrimitiveComponent Object Reference") (NormalImpulse :type "Vector Structure") (Hit :type "HitResult Structure (by ref)"))
  (bind _returnvalue (* (`self.SwingSpeed`) 50.0))
  (bind _asbp_tennis_ball (cast `/Game/TableTennis/Blueprints/BP_TennisBall` OtherActor))
  (`KismetSystemLibrary.PrintText` (`KismetTextLibrary.Conv_DoubleToText` _returnvalue "HalfToEven"))
  (bind (_tossvelocity _returnvalue_2) (`GameplayStatics.BlueprintSuggestProjectileVelocity` (`self.K2_GetActorLocation` _asbp_tennis_ball) (`self.K2_GetActorLocation` (`self.NewVar`)) _returnvalue 0.0 "DoNotTrace" 0.0 true true))
  (if _returnvalue_2
    (`PrimitiveComponent.SetPhysicsLinearVelocity` (`/Game/TableTennis/Blueprints/BP_TennisBall.BallMesh` _asbp_tennis_ball) _tossvelocity false "None")))

(fn `UserConstructionScript`)