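; Target spawner for a bow shooting range that also runs a timed scoring round.
; A looping timer spawns BP_Target actors at random points inside the SpawnArea box, capped at a few at once.
; StartGame clears targets, resets score and clock, and gives new targets a limited lifespan while Tick counts down.
; EndGame clears targets, swaps the time widget for the final score and resumes idle spawning.
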(event `self.ReceiveBeginPlay`
  (`SceneComponent.SetVisibility` (`self.ScoreWidget`) false false)
  (`SceneComponent.SetVisibility` (`self.TimeWidget`) false false)
  (bind _returnvalue (`KismetSystemLibrary.K2_SetTimer` null "Spawn Target" 1.0 true))
  (set `self.GeneralTimer` _returnvalue))

(event `self.ReceiveTick`
  (params (DeltaSeconds :type "Float (single-precision)"))
  (if (`self.Is Start`)
    (`self.Update Current Time` DeltaSeconds)
    (if (<= (`self.CurrentTime`) 0.0)
      (`self.End Game`))))

(fn `End Game`
  (bind _scorewidget (`self.ScoreWidget`))
  (set `self.Is Start` false)
  (`KismetSystemLibrary.K2_ClearAndInvalidateTimerHandle` (`self.StartTimer`))
  (bind _outactors (`GameplayStatics.GetAllActorsOfClass` "/Game/Bow/Blueprints/BP_Target.BP_Target_C"))
  (`self.K2_DestroyActor` _outactors)
  (`SceneComponent.SetVisibility` (`self.TimeWidget`) false false)
  (`SceneComponent.SetVisibility` _scorewidget true false)
  (bind _aswb_score (cast `/Game/Bow/Widget/WB_Score` (`WidgetComponent.GetUserWidgetObject` _scorewidget)))
  (`TextBlock.SetText` (`/Game/Bow/Widget/WB_Score.TB_Score` _aswb_score) (`KismetTextLibrary.Conv_DoubleToText` (`self.CurrentScore`) "HalfToEven"))
  (bind _returnvalue (`KismetSystemLibrary.K2_SetTimer` null "Spawn Target" 1.0 true))
  (set `self.GeneralTimer` _returnvalue))

(fn `Spawn Target`
  (bind _spawn_area (`self.Spawn_Area`))
  (bind _outactors (`GameplayStatics.GetAllActorsOfClass` "/Game/Bow/Blueprints/BP_Target.BP_Target_C"))
  (if (< (`KismetArrayLibrary.Array_Length` _outactors) 5)
    (bind _output_get (set `self.SpawnLocation` (`KismetMathLibrary.RandomPointInBoundingBox` (`SceneComponent.K2_GetComponentLocation` _spawn_area) (`BoxComponent.GetScaledBoxExtent` _spawn_area))))
    (bind _returnvalue (`|SpawnActorFromClass` "/Game/Bow/Blueprints/BP_Target.BP_Target_C" (`KismetMathLibrary.MakeTransform` _output_get) "AdjustIfPossibleButAlwaysSpawn" "OverrideRootScale" self null))
    (if (`self.Is Start`)
      (`self.SetLifeSpan` _returnvalue 10.0)
      (else
        (`self.SetLifeSpan` _returnvalue 0.0)))))

(fn `Start Game`
  (if (not (`self.Is Start`))
    (`KismetSystemLibrary.K2_ClearAndInvalidateTimerHandle` (`self.GeneralTimer`))
    (`KismetSystemLibrary.K2_ClearAndInvalidateTimerHandle` (`self.StartTimer`))
    (bind _outactors (`GameplayStatics.GetAllActorsOfClass` "/Game/Bow/Blueprints/BP_Target.BP_Target_C"))
    (`self.K2_DestroyActor` _outactors)
    (`SceneComponent.SetVisibility` (`self.ScoreWidget`) false false)
    (bind _returnvalue (`KismetSystemLibrary.K2_SetTimer` null "Spawn Target" 1.0 true))
    (set `self.StartTimer` _returnvalue)
    (set `self.CurrentScore` 0.0)
    (set `self.CurrentTime` (`self.MaxTime`))
    (bind _aswb_time (cast `/Game/Bow/Widget/WB_Time` (`WidgetComponent.GetUserWidgetObject` (`self.TimeWidget`))))
    (`TextBlock.SetText` (`/Game/Bow/Widget/WB_Time.TB_MaxTime` _aswb_time) (`KismetTextLibrary.Conv_DoubleToText` (`self.MaxTime`) "HalfToEven"))
    (`self.Update Score`)
    (`SceneComponent.SetVisibility` (`self.TimeWidget`) true false)
    (set `self.Is Start` true)))

(fn `Update Current Time`
  (params (`Delta Time` :type "Float (double-precision)"))
  (bind _output_get (set `self.CurrentTime` (- (`self.CurrentTime`) `Delta Time`)))
  (bind _aswb_time (cast `/Game/Bow/Widget/WB_Time` (`WidgetComponent.GetUserWidgetObject` (`self.TimeWidget`))))
  (`TextBlock.SetText` (`/Game/Bow/Widget/WB_Time.TB_CurrentTime` _aswb_time) (`KismetTextLibrary.Conv_Int64ToText` (`KismetMathLibrary.Conv_DoubleToInt64` _output_get))))

(fn `Update Score`
  (bind _aswb_time (cast `/Game/Bow/Widget/WB_Time` (`WidgetComponent.GetUserWidgetObject` (`self.TimeWidget`))))
  (`TextBlock.SetText` (`/Game/Bow/Widget/WB_Time.TB_CurrentScore` _aswb_time) (`KismetTextLibrary.Conv_DoubleToText` (`self.CurrentScore`) "HalfToEven")))

(fn `UserConstructionScript`
  (`BoxComponent.SetBoxExtent` (`self.Spawn_Area`) (`self.In Box Extent`) true))