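; VR bow actor that is held through one grab component and drawn by grabbing its notch with a motion controller.
; While pulled, controller distance from the notch's rest point sets the ABP_Bow draw progress and fades in the preview arrow's opacity.
; Dropping the notch spawns a BP_Arrow with speed scaled by draw, then resets the notch.
; Tick then eases the string back while the bow is held.
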(event `self.ReceiveBeginPlay`)

(event `self.ReceiveTick`
  (params (DeltaSeconds :type "Float (single-precision)"))
  (if (`self.IsHeld`)
    (if (`self.IsPulling`)
      (`self.PullingString`)
      (else
        (`self.ReleaseString` DeltaSeconds)))))

(event `self.GC_Notch.OnGrabbed`
  (set `self.IsPulling` true)
  (if (not (`AudioComponent.IsPlaying` (`self.PullBackAudio`)))
    (`AudioComponent.FadeIn` (`self.PullBackAudio`) 1.0 1.0 0.0 "Linear")))

(event `self.GC_Notch.OnDropped`
  (`self.SpawnArrow`)
  (set `self.IsPulling` false)
  (`self.NotchBack`))

(event `self.GrabComponent.OnGrabbed`
  (if (not (`self.IsHeld`))
    (set `self.IsHeld` true)))

(event `self.GrabComponent.OnDropped`
  (if (`self.IsHeld`)
    (set `self.IsHeld` false)))

(fn `NotchBack`
  (bind _notchmesh (`self.NotchMesh`))
  (`SceneComponent.K2_DetachFromComponent` _notchmesh "KeepWorld" "KeepWorld" "KeepWorld" true)
  (`SceneComponent.K2_SetWorldTransform` _notchmesh (`SceneComponent.K2_GetComponentToWorld` (`self.NotchOriginalMesh`)) false false)
  (`SceneComponent.K2_AttachToComponent` _notchmesh (`self.SkeletalMeshComponent`) "None" "KeepWorld" "KeepWorld" "KeepWorld" true))

(fn `PullingString`
  (bind _motioncontrollerref (`/Game/VRTemplate/Blueprints/GrabComponent.MotionControllerRef` (`self.GC_Notch`)))
  (if (`KismetSystemLibrary.IsValid` _motioncontrollerref)
    (if (`self.IsPulling`)
      (bind _asabp_bow (cast `/Game/Bow/Meshes/ABP_Bow` (`SkeletalMeshComponent.GetAnimInstance` (`self.SkeletalMeshComponent`))))
      (bind _output_get (set `/Game/Bow/Meshes/ABP_Bow.Current Slider Progress` (/ (`KismetMathLibrary.FClamp` (`KismetMathLibrary.VSize` (- (`SceneComponent.K2_GetComponentLocation` _motioncontrollerref) (`SceneComponent.K2_GetComponentLocation` (`self.NotchOriginalMesh`)))) 0.0 40.0) 40.0) _asabp_bow))
      (`MeshComponent.SetScalarParameterValueOnMaterials` (`self.ArrowMesh`) "Opacity" _output_get))))

(fn `ReleaseString`
  (params (DeltaTime :type "Float (double-precision)"))
  (bind _asabp_bow (cast `/Game/Bow/Meshes/ABP_Bow` (`SkeletalMeshComponent.GetAnimInstance` (`self.SkeletalMeshComponent`))))
  (set `/Game/Bow/Meshes/ABP_Bow.Current Slider Progress` (`KismetMathLibrary.FMax` (- (`/Game/Bow/Meshes/ABP_Bow.Current Slider Progress` _asabp_bow) (* DeltaTime 10.0))) _asabp_bow)
  (`MeshComponent.SetScalarParameterValueOnMaterials` (`self.ArrowMesh`) "Opacity" 0.0))

(fn `SpawnArrow`
  (bind _arrowforspawn (`self.ArrowForSpawn`))
  (bind _asabp_bow (cast `/Game/Bow/Meshes/ABP_Bow` (`SkeletalMeshComponent.GetAnimInstance` (`self.SkeletalMeshComponent`))))
  (bind _returnvalue (`|SpawnActorFromClass` "/Game/Bow/Blueprints/BP_Arrow.BP_Arrow_C" (`SceneComponent.K2_GetComponentToWorld` _arrowforspawn) "Undefined" "OverrideRootScale" null (`GameplayStatics.GetPlayerPawn` 0)))
  (`/Game/Bow/Blueprints/BP_Arrow.SetSpeed` _returnvalue (+ (`self.BaseSpeed`) (* (`/Game/Bow/Meshes/ABP_Bow.Current Slider Progress` _asabp_bow) 1000.0)) (`SceneComponent.GetForwardVector` _arrowforspawn))
  (`AudioComponent.Play` (`/Game/Bow/Blueprints/BP_Arrow.Audio` _returnvalue) 0.0))

(fn `UserConstructionScript`)