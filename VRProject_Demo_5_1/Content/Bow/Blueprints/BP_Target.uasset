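; BP_Target is an archery target actor that is destroyed when a BP_Arrow overlaps any of its three rings or its center.
; The construction script picks a random scale and a behavior: horizontal movement, vertical movement or scale adjustment.
; On BeginPlay, a timeline with randomized play rate lerps the mesh toward a random offset or one and a half times its base scale, according to that behavior.
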(event `self.ReceiveBeginPlay`
  (bind _returnvalue (`KismetMathLibrary.RandomFloatInRange` 100.0 250.0))
  (bind _sm_target (`self.SM_Target`))
  (bind _actorscale (`self.ActorScale`))
  (bind _returnvalue_2 (* _actorscale 1.5))
  (switch `/Game/Bow/Enum/E_TargetBehavior` (`self.TargetBehavior`)
    (:`NewEnumerator1`
      (set `self.DestinationLocation` (`KismetMathLibrary.MakeVector` _returnvalue)))
    (:`NewEnumerator2`
      (set `self.DestinationLocation` (`KismetMathLibrary.MakeVector` 0.0 0.0 _returnvalue)))
    (:`NewEnumerator3`
      _))
  (`TimelineComponent.SetPlayRate` (`self.T_Move`) (/ 1.0 (`KismetMathLibrary.RandomFloatInRange` 1.5 3.0)))
  (bind (_direction _alpha) (`Timeline|T_Move` :!via `PlayFromStart`)
    (:`Update`
      (switch `/Game/Bow/Enum/E_TargetBehavior` (`self.TargetBehavior`)
        (:`NewEnumerator1`
          (`SceneComponent.K2_SetRelativeLocation` _sm_target (`KismetMathLibrary.VLerp` (0.0 0.0 0.0) (`self.DestinationLocation`) _alpha) false false :!label _label))
        (:`NewEnumerator2`
          (goto _label))
        (:`NewEnumerator3`
          (`SceneComponent.SetWorldScale3D` _sm_target (`KismetMathLibrary.VLerp` (`KismetMathLibrary.MakeVector` _actorscale _actorscale _actorscale) (`KismetMathLibrary.MakeVector` _returnvalue_2 _returnvalue_2 _returnvalue_2) _alpha)))))))

(event `self.Ring1.OnComponentBeginOverlap`
  (params (OverlappedComponent :type "PrimitiveComponent Object Reference") (OtherActor :type "Actor Object Reference") (OtherComp :type "PrimitiveComponent Object Reference") (OtherBodyIndex :type Integer) (bFromSweep :type Boolean) (SweepResult :type "HitResult Structure (by ref)"))
  (cast `/Game/Bow/Blueprints/BP_Arrow` OtherActor)
  (`self.K2_DestroyActor`))

(event `self.Ring2.OnComponentBeginOverlap`
  (params (OverlappedComponent :type "PrimitiveComponent Object Reference") (OtherActor :type "Actor Object Reference") (OtherComp :type "PrimitiveComponent Object Reference") (OtherBodyIndex :type Integer) (bFromSweep :type Boolean) (SweepResult :type "HitResult Structure (by ref)"))
  (cast `/Game/Bow/Blueprints/BP_Arrow` OtherActor)
  (`self.K2_DestroyActor`))

(event `self.Ring3.OnComponentBeginOverlap`
  (params (OverlappedComponent :type "PrimitiveComponent Object Reference") (OtherActor :type "Actor Object Reference") (OtherComp :type "PrimitiveComponent Object Reference") (OtherBodyIndex :type Integer) (bFromSweep :type Boolean) (SweepResult :type "HitResult Structure (by ref)"))
  (cast `/Game/Bow/Blueprints/BP_Arrow` OtherActor)
  (`self.K2_DestroyActor`))

(event `self.Center.OnComponentBeginOverlap`
  (params (OverlappedComponent :type "PrimitiveComponent Object Reference") (OtherActor :type "Actor Object Reference") (OtherComp :type "PrimitiveComponent Object Reference") (OtherBodyIndex :type Integer) (bFromSweep :type Boolean) (SweepResult :type "HitResult Structure (by ref)"))
  (cast `/Game/Bow/Blueprints/BP_Arrow` OtherActor)
  (`self.K2_DestroyActor`))

(fn `UserConstructionScript`
  (bind _output_get (set `self.ActorScale` (`KismetMathLibrary.RandomFloatInRange` 0.4 0.8)))
  (`SceneComponent.SetWorldScale3D` (`self.SM_Target`) (`KismetMathLibrary.MakeVector` _output_get _output_get 1.0))
  (set `self.TargetBehavior` (cast `/Game/Bow/Enum/E_TargetBehavior` (`KismetMathLibrary.Conv_IntToByte` (`KismetMathLibrary.RandomIntegerInRange` 1 3)))))